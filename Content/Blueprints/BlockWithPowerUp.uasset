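; Block actor that releases a power-up when the player's ThirdPersonCharacter overlaps its box trigger.
; The overlap adds points to the score on ThirdPersonGameMode and spawns a PowerUp at the SpawnLocation component's transform.
; After a very short delay, the block destroys itself.
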(event `self.Box.OnComponentBeginOverlap`
  (params (OverlappedComponent :type "PrimitiveComponent Object Reference") (OtherActor :type "Actor Object Reference") (OtherComp :type "PrimitiveComponent Object Reference") (OtherBodyIndex :type Integer) (bFromSweep :type Boolean) (SweepResult :type "HitResult Structure (by ref)"))
  (cast `/Game/Blueprints/ThirdPersonCharacter` OtherActor)
  (bind _asthird_person_game_mode (cast `/Game/Blueprints/ThirdPersonGameMode` (`GameplayStatics.GetGameMode`)))
  (set `/Game/Blueprints/ThirdPersonGameMode.GMScore` (+ (`/Game/Blueprints/ThirdPersonGameMode.GMScore` _asthird_person_game_mode) 2) _asthird_person_game_mode)
  (`|SpawnActorFromClass` "/Game/Blueprints/PowerUp.PowerUp_C" (`SceneComponent.K2_GetComponentToWorld` (`self.SpawnLocation`)) "Undefined" "OverrideRootScale" null null)
  (`KismetSystemLibrary.Delay` 0.01)
  (`self.K2_DestroyActor`))

(fn `UserConstructionScript`)